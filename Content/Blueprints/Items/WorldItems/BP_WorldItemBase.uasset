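; BP_WorldItemBase is a base Blueprint for items placed in the world that can be outlined and expose pickup data.
; On BeginPlay it traces 1000 units down against one object type and moves itself to the hit location, without checking for a hit.
; Init functions store ID, SN, type, name, UI prefix, icon and mesh.
; Outlining toggles the mesh's custom depth, and GetPickupData returns icon, name and a zero amount.
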(event `self.ReceiveBeginPlay`
  (bind (_returnvalue_x _returnvalue_y _returnvalue_z) (`KismetMathLibrary.BreakVector` (`self.K2_GetActorLocation`)))
  (`parent.ReceiveBeginPlay`)
  (bind _outhit (`KismetSystemLibrary.LineTraceSingleForObjects` :`Start` (`self.K2_GetActorLocation`) :`End` (`KismetMathLibrary.MakeVector` _returnvalue_x _returnvalue_y (+ _returnvalue_z -1000.0)) :`ObjectTypes` (`|MakeArray` "ObjectTypeQuery7" :!type "EObjectTypeQuery Enum") :`DrawTime` 999.0))
  (`self.K2_SetActorLocation` (`.Location` (`GameplayStatics.BreakHitResult` _outhit))))

(fn `EnableOutline`
  (params (bIsEnabled :type Boolean))
  (`PrimitiveComponent.SetRenderCustomDepth` (`self.StaticMesh`) bIsEnabled))

(fn `GetPickupData`
  (returns (ItemIcon :type "Texture2D Object Reference") (ItemName :type Text) (Amount :type Integer))
  (return (`self.ItemIcon`) (`self.ItmeName`) 0))

(fn `InitSpawnData`
  (params (ID :type Name) (SN :type String))
  (set `self.ID` ID)
  (set `self.SN` SN))

(fn `InitWorldItemBaseData`
  (params (ItemType :type "/Game/Blueprints/Datas/Enum/Item/E_ItemType Enum" :default "NewEnumerator0") (ItemName :type Text) (UIPrefix :type "/Game/Blueprints/Datas/Enum/Item/E_UIPrefix Enum" :default "NewEnumerator0") (StaticMesh :type "StaticMesh Object Reference") (ItemIcon :type "Texture2D Object Reference"))
  (set `self.ItemType` ItemType)
  (set `self.ItmeName` ItemName)
  (set `self.UIPrefix` UIPrefix)
  (`StaticMeshComponent.SetStaticMesh` (`self.StaticMesh`) StaticMesh)
  (set `self.ItemIcon` ItemIcon))

(fn `UserConstructionScript`
  (`parent.UserConstructionScript`))