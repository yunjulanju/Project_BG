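; BP_Player is the player character Blueprint, providing movement, look input and a free-look mode.
; Move applies input along yaw-only forward or right vectors, while InputTurn and InputLookUp drive controller yaw and pitch.
; FreeLook saves control rotation and releases yaw-following on press; on release, a timeline lerps back by the shortest path, then restores it.
; A walk-speed clamp in Move is unconnected and never runs.
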(event `OnFreeLookEnded`
  ; 호출 부
  (bind (_direction _alpha) (`Timeline|Timeline` :!via `PlayFromStart`)
    (:`Update`
      (`Controller.SetControlRotation` (`self.GetController`) (`KismetMathLibrary.RLerp` (`self.FreeLookEndRotation`) (`self.FreeLookStartRotation`) _alpha true)))
    (:`Finished`
      (set `self.bUseControllerRotationYaw` true))))

(fn `FreeLook`
  (params (bIsPressed :type Boolean))
  (bind _returnvalue (`self.GetControlRotation`))
  (if bIsPressed
    (set `self.FreeLookStartRotation` _returnvalue)
    (set `self.bUseControllerRotationYaw` false)
    (else
      (set `self.FreeLookEndRotation` _returnvalue)
      (`self.OnFreeLookEnded`))))

(fn `InputLookUp`
  (params (YAxis :type "Float (double-precision)"))
  (`self.AddControllerPitchInput` YAxis))

(fn `InputTurn`
  (params (XAxis :type "Float (double-precision)"))
  (`self.AddControllerYawInput` XAxis))

(fn `Move`
  (params (bIsForward :type Boolean) (AxisValue :type "Float (double-precision)"))
  (locals (MaxSpeed :type "Float (double-precision)" :default 600.0) (Speed :type "Float (double-precision)" :default 5.0))
  (bind _axisvalue (`local.AxisValue`))
  (bind _yawonlyrotator (`/Game/Blueprints/Util/MathUtils.GetYawOnlyRotation` self))
  (if bIsForward
    (`self.AddMovementInput` (`KismetMathLibrary.GetForwardVector` _yawonlyrotator) _axisvalue)
    (else
      (`self.AddMovementInput` (`KismetMathLibrary.GetRightVector` _yawonlyrotator) _axisvalue))))

(fn `UserConstructionScript`)