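; BP_PlayerController is the player controller that relays movement and look input to the player character.
; On BeginPlay it casts the first player character to BP_Player and caches the reference.
; The Turn and LookUp axis events call that character's InputTurn and InputLookUp, while MoveForward and MoveRight share its Move function, distinguished by an IsForward flag.
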(event `self.ReceiveBeginPlay`
  (bind _asbp_player (cast `/Game/Blueprints/Character/BP_Player` (`GameplayStatics.GetPlayerCharacter` 0)))
  (set `self.BPPlayer` _asbp_player))

(event `InputAxis|MoveForward`
  (params (AxisValue :type "Float (single-precision)"))
  (`/Game/Blueprints/Character/BP_Player.Move` (`self.BPPlayer`) true AxisValue))

(event `InputAxis|Turn`
  (params (AxisValue :type "Float (single-precision)"))
  (`/Game/Blueprints/Character/BP_Player.InputTurn` (`self.BPPlayer`) AxisValue))

(event `InputAxis|MoveRight`
  (params (AxisValue :type "Float (single-precision)"))
  (`/Game/Blueprints/Character/BP_Player.Move` (`self.BPPlayer`) false AxisValue))

(event `InputAxis|LookUp`
  (params (AxisValue :type "Float (single-precision)"))
  (`/Game/Blueprints/Character/BP_Player.InputLookUp` (`self.BPPlayer`) AxisValue))

(fn `UserConstructionScript`)